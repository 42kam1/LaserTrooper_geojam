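; Base switch Blueprint that the player toggles by interacting, notifying its AffectedActors.
; On BeginPlay it binds to the player trooper's interact event and responds only when it is the interacted actor.
; Each toggle sends pressed or unpressed messages, plays a sound and drives a timeline forward or back to pitch the switch axis from its initial rotation.
; The Pressed flag runs inverted: the pressed message fires as it becomes false.
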(event Custom|InteractedWith
  (params (NewParam :type Actor%20Object%20Reference))
  (bind _initrot (Variables|Default|GetInitRot))
  (bind _affectedactors (Variables|Default|GetAffectedActors))
  ;[1 1 1] bind interaction event
  (if (== NewParam self)
    ;[1 1 1] switch ON/OFF
    (if (Variables|Default|GetPressed)
      (Variables|Default|SetPressed false)
      (Class|ButtonInterface|ButtonPressed(Message) _affectedactors)
      (Audio|PlaySound2D "/Game/StarterContent/Audio/Explosion01.Explosion01" 1.0 1.0 0.0 0 0)
      ;[1 1 1] visual part
      (bind _newtrack_0 (Timeline|Timeline_0 Play)
        (:Update
          (Transformation|SetWorldRotation (Variables|Default|GetSwitchAxis) (Math|Rotator|MakeRotator (.roll _initrot) (+ (.pitch _initrot) _newtrack_0) (.yaw _initrot)) false false)))
      (else
        (Variables|Default|SetPressed true)
        (Class|ButtonInterface|ButtonUnpressed(Message) _affectedactors)
        (Audio|PlaySound2D "/Game/StarterContent/Audio/Explosion01.Explosion01" 1.0 1.0 0.0 0 0)
        (Timeline|Timeline_0 Reverse)))))

(event EventBeginPlay
  (Variables|Default|SetInitRot (Transformation|GetWorldRotation (Variables|Default|GetSwitchAxis)))
  ;[1 1 1] bind interaction event
  (bind _ascharacter_trooper_bp (Utilities|Casting|CastToCharacterTrooperBP (Game|Player|GetPlayerPawn 0)))
  (EventDispatchers|BindEventtoInterract _ascharacter_trooper_bp (delegate Custom|InteractedWith)))

(fn ConstructionScript)