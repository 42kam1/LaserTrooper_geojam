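; GeneratorBP is a one-shot destructible generator that triggers other actors when the player's damage-trigger event fires.
; On BeginPlay it casts the player pawn to CharacterTrooperBP and binds ButtonPress to that event.
; ButtonPress passes through a DoOnce, sends the ButtonPressed message to AffectedActors, plays an explosion sound and swaps the Working component for the Broken one.
; The event's parameter is unused, so the handler does not check what was hit.
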(event Custom|ButtonPress
  (params (NewParam :type Actor%20Object%20Reference))
  ;[1 1 1] bind interaction event
  (Utilities|FlowControl|DoOnce false
    (:Completed
      (Class|ButtonInterface|ButtonPressed(Message) (Variables|Default|GetAffectedActors))
      (Audio|PlaySound2D "/Game/StarterContent/Audio/Explosion01.Explosion01" 1.0 1.0 0.0 0 0)
      ;[1 1 1] is now broken
      (Rendering|SetVisibility (Variables|Default|GetBroken) true false)
      (Rendering|SetVisibility (Variables|Default|GetWorking) false false))))

(event EventBeginPlay
  ;[1 1 1] bind interaction event
  (bind _ascharacter_trooper_bp (Utilities|Casting|CastToCharacterTrooperBP (Game|Player|GetPlayerPawn 0)))
  (EventDispatchers|BindEventtoDamageTrigger _ascharacter_trooper_bp (delegate Custom|ButtonPress)))

(fn ConstructionScript)