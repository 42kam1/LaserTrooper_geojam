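; ButtonBaseBP is an interactive toggle button that switches other actors on and off.
; On BeginPlay it binds to the CharacterTrooperBP player pawn's interact event and responds only when the event targets this button.
; Each press flips the OnOff state, sends a pressed or unpressed message to AffectedActors and plays a sound.
; A dynamic material instance created in the construction script recolors the button green for on, red for off.
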(event Custom|ButtonPress
  (params (NewParam :type Actor%20Object%20Reference))
  (bind _affectedactors (Variables|Default|GetAffectedActors))
  ;[1 1 1] bind interaction event
  (if (== NewParam self)
    ;[1 1 1] switch ON/OFF
    (if (Variables|Default|GetOn\Off)
      (Variables|Default|SetOn\Off false)
      (Class|ButtonInterface|ButtonUnpressed(Message) _affectedactors)
      (Audio|PlaySound2D "/Game/StarterContent/Audio/Fire_Sparks01.Fire_Sparks01" 1.0 1.0 0.0 0 0)
      ;[1 1 1] visual part
      (Rendering|Material|SetVectorParameterValue (Variables|Default|GetButtonColor) "ButtonColor" "(R=1.000000,G=0.000000,B=0.006724,A=1.000000)" :!class /Script/Engine.MaterialInstanceDynamic)
      (else
        (Variables|Default|SetOn\Off true)
        (Class|ButtonInterface|ButtonPressed(Message) _affectedactors)
        (Audio|PlaySound2D "/Game/StarterContent/Audio/Fire_Sparks01.Fire_Sparks01" 1.0 1.0 0.0 0 0)
        (Rendering|Material|SetVectorParameterValue (Variables|Default|GetButtonColor) "ButtonColor" "(R=0.000000,G=1.000000,B=0.236359,A=1.000000)" :!class /Script/Engine.MaterialInstanceDynamic)))))

(event EventBeginPlay
  ;[1 1 1] bind interaction event
  (bind _ascharacter_trooper_bp (Utilities|Casting|CastToCharacterTrooperBP (Game|Player|GetPlayerPawn 0)))
  (EventDispatchers|BindEventtoInterract _ascharacter_trooper_bp (delegate Custom|ButtonPress)))

(fn ConstructionScript
  (bind _returnvalue (Rendering|Material|CreateDynamicMaterialInstance (Variables|Default|GetButton) 0 "/Game/A/Materials/Button_Inst.Button_Inst" "None" :!class /Script/Engine.PrimitiveComponent))
  (Variables|Default|SetButtonColor _returnvalue))