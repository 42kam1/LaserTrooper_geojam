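; DoorBaseBP is a door Blueprint that slides open and closed in response to button press and unpress events.
; It records the door's world location on BeginPlay.
; A timeline plays on press and reverses on release, adding its track value to the stored Y coordinate to move the door along the world Y axis without sweeping.
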(event EventButtonPressed
  (bind _initialdoorloca (Variables|Default|GetInitialDoorLoca))
  (bind (_x _y _z) (Math|Vector|BreakVector _initialdoorloca))
  (bind _newtrack_0 (Timeline|Timeline_0 Play)
    (:Update
      (Transformation|SetWorldLocation (Variables|Default|GetDoor) (Math|Vector|MakeVector _x (+ _newtrack_0 _y) _z) false false))))

(event EventBeginPlay
  (Variables|Default|SetInitialDoorLoca (Transformation|GetWorldLocation (Variables|Default|GetDoor))))

(event EventButtonUnpressed
  (bind _initialdoorloca (Variables|Default|GetInitialDoorLoca))
  (bind (_x _y _z) (Math|Vector|BreakVector _initialdoorloca))
  (bind _newtrack_0 (Timeline|Timeline_0 Reverse)
    (:Update
      (Transformation|SetWorldLocation (Variables|Default|GetDoor) (Math|Vector|MakeVector _x (+ _newtrack_0 _y) _z) false false))))

(fn ConstructionScript)